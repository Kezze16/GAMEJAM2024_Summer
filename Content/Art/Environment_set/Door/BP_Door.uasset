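; BP_Door is a three-panel sliding door actor that opens when its OpenDoor event is called.
; OpenDoor fires separate events that slide the left and right panels outward and the top panel upward, each with an eased MoveComponentTo over the same duration.
; It then disables collision on the whole actor immediately, and the file contains no closing logic or trigger.
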(event `OpenLeft`
  (bind _door_left (`self.Door_left`))
  ;[1 1 1] Open Doors
  (`KismetSystemLibrary.MoveComponentTo` _door_left (+ (`SceneComponent.RelativeLocation` _door_left) (-175.0 0.0 0.0)) (struct) false true 1.5))

(event `Open Right`
  (bind _door_right (`self.Door_right`))
  ;[1 1 1] Open Doors
  (`KismetSystemLibrary.MoveComponentTo` _door_right (+ (`SceneComponent.RelativeLocation` _door_right) (175.0 0.0 0.0)) (struct) false true 1.5))

(event `Open Top`
  (bind _door_top (`self.Door_top`))
  ;[1 1 1] Open Doors
  (`KismetSystemLibrary.MoveComponentTo` _door_top (+ (`SceneComponent.RelativeLocation` _door_top) (0.0 0.0 75.0)) (struct) false true 1.5))

(event `Open Door`
  (`self.OpenLeft`)
  (`self.Open Right`)
  (`self.Open TOp`)
  (`self.SetActorEnableCollision` self false))

(fn `UserConstructionScript`)