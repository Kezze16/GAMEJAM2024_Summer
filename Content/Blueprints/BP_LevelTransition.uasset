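; Level transition trigger that sends the game to a randomly chosen next level when an actor overlaps its box.
; The overlap calls GoToNextLevel, which disables input if the overlapping actor is the player character, though the transition itself runs either way.
; It shows a WBP_Transition fade-out widget, waits briefly for the fade, then opens a random entry from the Levels array.
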(event `self.Box.OnComponentBeginOverlap`
  (params (OverlappedComponent :type "PrimitiveComponent Object Reference") (OtherActor :type "Actor Object Reference") (OtherComp :type "PrimitiveComponent Object Reference") (OtherBodyIndex :type Integer) (bFromSweep :type Boolean) (SweepResult :type "HitResult Structure (by ref)"))
  (`self.GoToNextLevel`))

(event `GoToNextLevel`
  (bind _asbp_player_character (cast `/Game/Character/BP_Player_Character` (stale `self.Box.OnComponentBeginOverlap` OtherActor))
    (:`then`
      (`self.DisableInput` _asbp_player_character null))
    (:`CastFailed`
      _))
  (bind _returnvalue (`|CreateWidget` "/Game/Blueprints/WBP_Transition.WBP_Transition_C"))
  (`UserWidget.AddToViewport` _returnvalue 0)
  (`/Game/Blueprints/WBP_Transition.FadeOut` _returnvalue)
  (`KismetSystemLibrary.Delay` 1.6)
  (`GameplayStatics.OpenLevelBySoftObjectPtr` (`KismetArrayLibrary.Array_Random` (`self.Levels`))))

(fn `UserConstructionScript`)