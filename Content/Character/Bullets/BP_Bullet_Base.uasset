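; Base bullet actor that flies forward and explodes for area damage on overlap or at maximum range.
; A transferred health amount becomes its Damage, which also scales speed, travel distance and blast radius.
; Tick moves it with a swept offset and checks range; overlaps deal direct damage, then call Deploy.
; Deploy runs a debug-drawn sphere trace, damages hit actors and destroys the bullet.
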(event `DistanceToKill`
  ;[1 1 1] Distance To Kill
  (if (>= (`KismetMathLibrary.Vector_Distance` (`self.StartLocation`) (`self.K2_GetActorLocation`)) (* (`self.MaxDistance`) (`self.Damage`)))
    (`self.Deploy`)))

(event `self.ReceiveBeginPlay`
  (set `self.StartLocation` (`self.K2_GetActorLocation`)))

(event `MoveProjectile`
  ;[1 1 1] Move
  (`self.K2_AddActorWorldOffset` (* (`self.GetActorForwardVector`) (* (`self.Speed`) (`self.Damage`))) true))

(event `self.ReceiveTick`
  (params (DeltaSeconds :type "Float (single-precision)"))
  (`self.MoveProjectile`)
  (`self.DistanceToKill`))

(event `self.Sphere.OnComponentBeginOverlap`
  (params (OverlappedComponent :type "PrimitiveComponent Object Reference") (OtherActor :type "Actor Object Reference") (OtherComp :type "PrimitiveComponent Object Reference") (OtherBodyIndex :type Integer) (bFromSweep :type Boolean) (SweepResult :type "HitResult Structure (by ref)"))
  (message `/Game/Hugo/Interfaces/BI_Damage.DealDamage` OtherActor (`self.Damage`))
  (`self.Deploy`))

(event `/Game/Hugo/Interfaces/BI_Health.TransferHealthAmount`
  (params (HealthAmount :type "Float (double-precision)"))
  (set `self.Damage` HealthAmount))

(event `/Game/Hugo/Interfaces/BI_Damage.DealDamage`
  (params (AmountOfDamage :type "Float (double-precision)"))
  (`KismetSystemLibrary.Delay` 0.1 :!label _label)
  (`self.Deploy`))

(event `/Game/Hugo/Interfaces/BI_Damage.Explosion`
  (params (PotentialDamage :type "Float (double-precision)"))
  (goto _label))

(fn `Deploy`
  (bind _damage (`self.Damage`))
  (bind _returnvalue (`SceneComponent.K2_GetComponentLocation` (`self.Sphere`)))
  (bind _outhits (`KismetSystemLibrary.SphereTraceMulti` :`Start` _returnvalue :`End` _returnvalue :`Radius` (* (`self.Damage`) (`self.RadiusMultiplyer`)) :`TraceChannel` "TraceTypeQuery3" :`DrawDebugType` "ForDuration"))
  (if (`KismetArrayLibrary.Array_IsEmpty` _outhits)
    (`self.K2_DestroyActor`)
    (else
      (for _array_element _outhits
        (message `/Game/Hugo/Interfaces/BI_Damage.DealDamage` (`.HitActor` (`GameplayStatics.BreakHitResult` _array_element)) _damage)
        (`KismetSystemLibrary.PrintString` (`KismetStringLibrary.Conv_DoubleToString` _damage))
        (`self.K2_DestroyActor`)))))

(fn `UserConstructionScript`)