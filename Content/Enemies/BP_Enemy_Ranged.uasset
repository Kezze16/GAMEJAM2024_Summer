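; BP_Enemy_Ranged is a ranged enemy that constantly faces the player, closes to attack range and fires homing bullets.
; A looping timer issues AIMoveTo while not attacking, and arrival starts an attack with a cooldown.
; The attack scales the rocket through a timeline, then spawns an explosion effect and a bullet homing on the player's capsule.
; Damage goes through a health component, death explodes and destroys it, and the health bar faces the camera.
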(event `self.ReceiveTick`
  (params (DeltaSeconds :type "Float (single-precision)"))
  (`self.K2_SetActorRotation` (`KismetMathLibrary.FindLookAtRotation` (`self.K2_GetActorLocation`) (`self.K2_GetActorLocation` (`self.Target`))))
  (`self.RotateHealthBar`))

(event `self.ReceiveBeginPlay`
  (bind _returnvalue (`GameplayStatics.GetActorOfClass` "/Game/Character/BP_Player_Character.BP_Player_Character_C"))
  (set `self.Target` _returnvalue)
  (`KismetSystemLibrary.K2_SetTimerDelegate` (delegate `MoveTowardsTarget`) 0.5 true))

(event `MoveTowardsTarget`
  (bind _target (`self.Target`))
  (if (not (`self.Attacking`))
    (`|AIMoveTo` self (`self.K2_GetActorLocation` _target) _target (* (`self.AttackRadius`) 0.9)
      (:`OnSuccess`
        (`self.AttackEvent`)))))

(event `AttackEvent`
  (`|ExecutionSequence`
    (:`then_0`
      (set `self.Attacking` true)
      (bind (_direction _yscale _xscale) (`Timeline|Attack` :!via `PlayFromStart`)
        (:`Update`
          (`SceneComponent.SetRelativeScale3D` (`self.Rocket`) (`KismetMathLibrary.MakeVector` _xscale _xscale _yscale)))))
    (:`then_1`
      (`KismetSystemLibrary.Delay` 1.2)
      (`GameplayStatics.SpawnEmitterAtLocation` "/Game/StarterContent/Particles/P_Explosion.P_Explosion" (`SceneComponent.K2_GetComponentLocation` (`self.Aim`)) (struct) (0.5 0.5 0.5))
      (`|SpawnActorFromClass` "/Game/Enemies/BP_Enemy_Bullet.BP_Enemy_Bullet_C" (`SceneComponent.K2_GetComponentToWorld` (`self.Aim`)) "Undefined" "MultiplyWithRoot" null (`self.GetComponentByClass` (`self.Target`) "/Script/Engine.CapsuleComponent") null))
    (:`then_2`
      (`KismetSystemLibrary.Delay` (`self.AttackCooldown`))
      (set `self.Attacking` false))))

(event `/Game/Hugo/Interfaces/BI_Damage.DealDamage`
  (params (AmountOfDamage :type "Float (double-precision)"))
  (bind _enemy_healthcomponent (`self.Enemy_HealthComponent`))
  (`/Game/Enemies/Enemy_HealthComponent.Damage` _enemy_healthcomponent AmountOfDamage (`self.HealthBarWidget`))
  (if (<= (`/Game/Enemies/Enemy_HealthComponent.CurrentHealth` _enemy_healthcomponent) 0.0)
    (`self.Die`)))

(event `Die`
  (`GameplayStatics.SpawnEmitterAtLocation` "/Game/StarterContent/Particles/P_Explosion.P_Explosion" (`self.K2_GetActorLocation`) (struct) (2.0 2.0 2.0))
  (`self.K2_DestroyActor`))

(event `RotateHealthBar`
  (bind _healthbarwidget (`self.HealthBarWidget`))
  (`SceneComponent.K2_SetWorldRotation` _healthbarwidget (`KismetMathLibrary.FindLookAtRotation` (`SceneComponent.K2_GetComponentLocation` _healthbarwidget) (`SceneComponent.K2_GetComponentLocation` (`PlayerCameraManager.TransformComponent` (`GameplayStatics.GetPlayerCameraManager` 0)))) false false))

(fn `UserConstructionScript`)