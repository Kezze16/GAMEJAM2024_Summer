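; Enemy spawner that keeps spawning random enemies from its Enemies list on the ground within its box area.
; A self-calling delay loop sets the pace, while a timeline lerps the interval from StartSpawnRate to EndSpawnRate.
; Each spawn line-traces downward between randomly picked box points to find a location.
; It shows a sparks emitter there for a short warning delay, then spawns the enemy just above and removes the effect.
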(event `self.ReceiveBeginPlay`
  (set `self.CurrentSpawnRate` (`self.StartSpawnRate`))
  (`self.SpawnDelay`)
  (bind (_direction _alpha) (`Timeline|Timeline` :!via `PlayFromStart`)
    (:`Update`
      (set `self.CurrentSpawnRate` (`KismetMathLibrary.Lerp` (`self.StartSpawnRate`) (`self.EndSpawnRate`) _alpha)))))

(event `SpawnDelay`
  (`self.SpawnBeavo`)
  (`KismetSystemLibrary.Delay` (`self.CurrentSpawnRate`))
  (`self.SpawnDelay`))

(event `SpawnBeavo`
  (bind _returnvalue (`KismetMathLibrary.RandomPointInBoundingBox` (`self.K2_GetActorLocation`) (`BoxComponent.GetScaledBoxExtent` (`self.Box`))))
  (bind _outhit (`KismetSystemLibrary.LineTraceSingle` _returnvalue (+ _returnvalue (0.0 0.0 -1000.0)) "TraceTypeQuery1"))
  (bind _output_get (set `self.RandomPoint` (`.Location` (`GameplayStatics.BreakHitResult` _outhit))))
  (bind _returnvalue_2 (`GameplayStatics.SpawnEmitterAtLocation` "/Game/StarterContent/Particles/P_Sparks.P_Sparks" _output_get))
  (`KismetSystemLibrary.Delay` 2.0)
  (`|SpawnActorFromClass` (`KismetArrayLibrary.Array_Random` (`self.Enemies`)) (`KismetMathLibrary.MakeTransform` (+ (`self.RandomPoint`) (0.0 0.0 50.0))) "AdjustIfPossibleButAlwaysSpawn" "MultiplyWithRoot" null null)
  (`ActorComponent.K2_DestroyComponent` _returnvalue_2))

(fn `UserConstructionScript`)