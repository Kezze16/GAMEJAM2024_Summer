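; Boss enemy that hunts the player character and opens the win level when killed.
; A looping timer drives AI movement toward the player, while Tick turns the boss to face them and its health bar toward the camera.
; On arrival, a timeline scales Beavo, then a delayed sphere trace deals damage and fires a homing bullet per hit before cooldown.
; Damage feeds the health component; death triggers effects and a camera fade.
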(event `self.ReceiveTick`
  (params (DeltaSeconds :type "Float (single-precision)"))
  (bind (_returnvalue_roll _returnvalue_pitch _returnvalue_yaw) (`KismetMathLibrary.BreakRotator` (`KismetMathLibrary.FindLookAtRotation` (`self.K2_GetActorLocation`) (`self.K2_GetActorLocation` (`self.Target`)))))
  (`self.K2_SetActorRotation` (`KismetMathLibrary.MakeRotator` _returnvalue_roll 0.0 _returnvalue_yaw))
  (`self.RotateHealthBar`))

(event `self.ReceiveBeginPlay`
  (bind _returnvalue (`GameplayStatics.GetActorOfClass` "/Game/Character/BP_Player_Character.BP_Player_Character_C"))
  (set `self.Target` _returnvalue)
  (`KismetSystemLibrary.K2_SetTimerDelegate` (delegate `MoveTowardsTarget`) 0.5 true))

(event `MoveTowardsTarget`
  (bind _target (`self.Target`))
  (if (not (`self.Attacking`))
    (`|AIMoveTo` self (`self.K2_GetActorLocation` _target) _target (* (`self.AttackRadius`) 0.75)
      (:`OnSuccess`
        (`self.AttackEvent`)))))

(event `AttackEvent`
  (bind _returnvalue (`self.K2_GetActorLocation`))
  (bind _aim (`self.Aim`))
  (bind (_returnvalue_location _returnvalue_rotation) (`KismetMathLibrary.BreakTransform` (`SceneComponent.K2_GetComponentToWorld` _aim)))
  (bind _returnvalue_2 (`SceneComponent.K2_GetComponentLocation` _aim))
  (`|ExecutionSequence`
    (:`then_0`
      (set `self.Attacking` true)
      (bind (_direction _yscale _xscale) (`Timeline|Attack` :!via `PlayFromStart`)
        (:`Update`
          (`SceneComponent.SetRelativeScale3D` (`self.Beavo`) (`KismetMathLibrary.MakeVector` _xscale _xscale _yscale)))))
    (:`then_1`
      (`KismetSystemLibrary.Delay` 1.2)
      (`GameplayStatics.PlaySoundAtLocation` "/Game/Sound/Hazard/Explosion.Explosion" (`self.K2_GetActorLocation`) (struct) 1.0 1.0 0.0 null null null null)
      (`NiagaraFunctionLibrary.SpawnSystemAtLocation` "/Game/KTP_Effect/Particles/Fly/Expolison_08_01.Expolison_08_01" (`SceneComponent.K2_GetComponentLocation` (`self.Beavo`)) (struct :`Pitch` 90.0) (1.0 3.5 3.5))
      (bind _outhits (`KismetSystemLibrary.SphereTraceMulti` :`Start` _returnvalue :`End` _returnvalue :`Radius` (`self.AttackRadius`) :`TraceChannel` "TraceTypeQuery3" :`DrawTime` 1.0))
      (for _array_element _outhits
        (message `/Game/Hugo/Interfaces/BI_Damage.DealDamage` (`.HitActor` (`GameplayStatics.BreakHitResult` _array_element)) 1.0)
        (`GameplayStatics.PlaySoundAtLocation` "/Game/Sound/Enemy/RocketShot.RocketShot" _returnvalue_2 (struct) 1.0 1.0 0.0 null null null null)
        (`GameplayStatics.SpawnEmitterAtLocation` "/Game/StarterContent/Particles/P_Explosion.P_Explosion" _returnvalue_2 (struct) (0.5 0.5 0.5))
        (`|SpawnActorFromClass` "/Game/Enemies/BP_Enemy_Bullet.BP_Enemy_Bullet_C" (`KismetMathLibrary.MakeTransform` _returnvalue_location _returnvalue_rotation (2.0 2.0 2.0)) "Undefined" "MultiplyWithRoot" null (`self.GetComponentByClass` (`self.Target`) "/Script/Engine.CapsuleComponent") null)))
    (:`then_2`
      (`KismetSystemLibrary.Delay` (`self.AttackCooldown`))
      (set `self.Attacking` false))))

(event `self.DealDamage`
  (params (AmountOfDamage :type "Float (double-precision)"))
  (bind _enemy_healthcomponent (`self.Enemy_HealthComponent`))
  (`/Game/Enemies/Enemy_HealthComponent.Damage` _enemy_healthcomponent AmountOfDamage (`self.HealthBarWidget`))
  (if (<= (`/Game/Enemies/Enemy_HealthComponent.CurrentHealth` _enemy_healthcomponent) 0.0)
    (`GameplayStatics.PlaySound2D` "/Game/Sound/Player/Death.Death" 1.0 1.0 0.0 null null)
    (`self.Die`)))

(event `Die`
  (bind _returnvalue (`self.K2_GetActorLocation`))
  (if (not (`self.dead`))
    (set `self.dead` true)
    (`GameplayStatics.SpawnEmitterAtLocation` "/Game/StarterContent/Particles/P_Explosion.P_Explosion" _returnvalue (struct) (2.0 2.0 2.0))
    (`GameplayStatics.PlaySoundAtLocation` "/Game/Sound/Player/Death_Cue.Death_Cue" _returnvalue (struct) 1.0 1.0 0.0 null null null null)
    (`PlayerCameraManager.StartCameraFade` :`self` (`GameplayStatics.GetPlayerCameraManager` 0) :`ToAlpha` 2.0 :`Duration` 2.0 :`bShouldFadeAudio` true)
    (set `self.Attacking` true)
    (`|AIMoveTo` self (`self.K2_GetActorLocation`) null
      (:`then`
        (`KismetSystemLibrary.Delay` 3.0)
        (`GameplayStatics.OpenLevelBySoftObjectPtr` "/Game/Levels/L_Win.L_Win")))))

(event `RotateHealthBar`
  (bind _healthbarwidget (`self.HealthBarWidget`))
  (`SceneComponent.K2_SetWorldRotation` _healthbarwidget (`KismetMathLibrary.FindLookAtRotation` (`SceneComponent.K2_GetComponentLocation` _healthbarwidget) (`SceneComponent.K2_GetComponentLocation` (`PlayerCameraManager.TransformComponent` (`GameplayStatics.GetPlayerCameraManager` 0)))) false false))

(event `self.Explosion`
  (params (PotentialDamage :type "Float (double-precision)"))
  (`self.DealDamage` PotentialDamage))

(fn `UserConstructionScript`)