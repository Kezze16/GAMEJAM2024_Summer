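; Game mode that tracks the player's upgrades: stronger bullets, shield, speed boost and backwards bullet.
; Each upgrade event forwards a message to player character 0 and sets a flag, also storing the last percentage for bullets and speed.
; CheckUpgrades replays every flagged upgrade with its stored value, so the current character can receive them again.
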(event `self.StrongerBullets`
  (params (Procent :type "Float (double-precision)"))
  (bind _output_get (set `self.LastUpdatedStrongerBulletsProcent` Procent))
  (message `/Game/Hugo/Interfaces/BI_Upgrade.StrongerBullets` (`GameplayStatics.GetPlayerCharacter` 0) _output_get)
  (set `self.hasStrongerbullets` true))

(event `self.Shield`
  (message `/Game/Hugo/Interfaces/BI_Upgrade.Shield` (`GameplayStatics.GetPlayerCharacter` 0))
  (set `self.hasShield` true))

(event `self.SpeedBoost`
  (params (Procentege :type "Float (double-precision)"))
  (bind _output_get (set `self.LastUpdatedSpeedBoostProcent` Procentege))
  (message `/Game/Hugo/Interfaces/BI_Upgrade.SpeedBoost` (`GameplayStatics.GetPlayerCharacter` 0) _output_get)
  (set `self.hasSpeedBoost` true))

(event `self.BackwardsBullet`
  (message `/Game/Hugo/Interfaces/BI_Upgrade.BackwardsBullet` (`GameplayStatics.GetPlayerCharacter` 0))
  (set `self.hasBackwardBullet` true))

(event `self.CheckUpgrades`
  (`self.CheckStrongerBullets`)
  (`self.CheckShield`)
  (`self.CheckSpeedBoost`)
  (`self.Check Backward Bullet`))

(event `CheckStrongerBullets`
  (if (`self.hasStrongerbullets`)
    (`self.StrongerBullets` (`self.LastUpdatedStrongerBulletsProcent`))))

(event `CheckShield`
  (if (`self.hasShield`)
    (`self.Shield`)))

(event `CheckSpeedBoost`
  (if (`self.hasSpeedBoost`)
    (`self.SpeedBoost` (`self.LastUpdatedSpeedBoostProcent`))))

(event `Check Backward Bullet`
  (if (`self.hasBackwardBullet`)
    (`self.BackwardsBullet`)))

(fn `UserConstructionScript`)