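; BP_Heart is a health pickup that launches upward in a random horizontal direction when spawned and gives its health amount to the player.
; ProjectileMovement drives the launch, while a timeline scaled to a set duration eases RotatingMovement from its starting spin to an idle rate.
; A short delay sets the pickup sphere's radius; player overlap passes the externally set health amount through an interface message and destroys the heart.
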(event `ShootInRandomDirection`
  (bind (_returnvalue_x _returnvalue_y) (`KismetMathLibrary.BreakVector` (`SceneComponent.GetForwardVector` (`self.StaticMesh`))))
  (bind _returnvalue (`KismetMathLibrary.RandomFloatInRange` (`self.MinSpeed`) (`self.MaxSpeed`)))
  ;[0 1 0.4139] Shoot In Random Direction
  (`self.K2_SetActorRotation` (`KismetMathLibrary.MakeRotator` 0.0 0.0 (`KismetMathLibrary.RandomFloatInRange` 0.0 360.0)))
  (`ProjectileMovementComponent.SetVelocityInLocalSpace` (`self.ProjectileMovement`) (`KismetMathLibrary.MakeVector` (* _returnvalue_x _returnvalue) (* _returnvalue_y _returnvalue) 650.0)))

(event `self.ReceiveBeginPlay`
  (bind _slowdownrotation (`self.SlowDownRotation`))
  (`self.ShootInRandomDirection`)
  (`self.Set Sphere Radius`)
  (set `RotatingMovementComponent.RotationRate` (`self.StartingRotationRate`) (`self.RotatingMovement`))
  (`TimelineComponent.SetPlayRate` _slowdownrotation (/ (`TimelineComponent.GetTimelineLength` _slowdownrotation) (`self.TimeToSLowDOwnRotateRate`)))
  (`self.SlowDownRotationEvent`))

(event `/Game/Hugo/Interfaces/BI_Health.TransferHealthAmount`
  (params (HealthAmount :type "Float (double-precision)"))
  (set `self.HealthAmountToGive` HealthAmount))

(event `self.PickUpAreaCollision.OnComponentBeginOverlap`
  (params (OverlappedComponent :type "PrimitiveComponent Object Reference") (OtherActor :type "Actor Object Reference") (OtherComp :type "PrimitiveComponent Object Reference") (OtherBodyIndex :type Integer) (bFromSweep :type Boolean) (SweepResult :type "HitResult Structure (by ref)"))
  (if (== (`GameplayStatics.GetObjectClass` OtherActor) "/Game/Character/BP_Player_Character.BP_Player_Character_C")
    (message `/Game/Hugo/Interfaces/BI_Health.TransferHealthAmount` OtherActor (`self.HealthAmountToGive`))
    (`self.K2_DestroyActor`)))

(event `Set Sphere Radius`
  (`KismetSystemLibrary.Delay` 1.2)
  (`SphereComponent.SetSphereRadius` (`self.PickUpAreaCollision`) (`self.PickUpCpllisionRadious`) true))

(event `SlowDownRotationEvent`
  (bind (_direction _rotationlerp) (`Timeline|SlowDownRotation`)
    (:`Update`
      (set `RotatingMovementComponent.RotationRate` (`KismetMathLibrary.RLerp` (`self.StartingRotationRate`) (`self.IdleRotationRate`) _rotationlerp) (`self.RotatingMovement`)))))

(fn `UserConstructionScript`)