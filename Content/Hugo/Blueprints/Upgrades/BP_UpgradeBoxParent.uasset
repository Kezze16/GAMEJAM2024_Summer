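; Upgrade box pickup parent that grants the player one of four random upgrades: backwards bullet, speed boost, shield or stronger bullets.
; On BeginPlay it creates a hidden BW_Upgrade widget, spawns a BP_Quest at its arrow and rolls the upgrade.
; The first player overlap, gated by DoOnce, notifies the game mode of the upgrade and shows its description for a timed delay.
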(event `self.ReceiveBeginPlay`
  (bind _arrow (`self.Arrow`))
  (`self.SetUpWidgets`)
  (`|SpawnActorFromClass` "/Game/Blueprints/BP_Quest.BP_Quest_C" (`KismetMathLibrary.MakeTransform` (`SceneComponent.K2_GetComponentLocation` _arrow) (`SceneComponent.K2_GetComponentRotation` _arrow)) "Undefined" "MultiplyWithRoot" null null)
  (switch `int` (`KismetMathLibrary.RandomIntegerInRange` 0 3)
    (:`Default`
      (set `self.ListOfUpgrades` "NewEnumerator1" :!label _label))
    (:`0`
      (set `self.ListOfUpgrades` "NewEnumerator0"))
    (:`1`
      (goto _label))
    (:`2`
      (set `self.ListOfUpgrades` "NewEnumerator3"))
    (:`3`
      (set `self.ListOfUpgrades` "NewEnumerator4"))))

(event `self.PickUpCollision.OnComponentBeginOverlap`
  (params (OverlappedComponent :type "PrimitiveComponent Object Reference") (OtherActor :type "Actor Object Reference") (OtherComp :type "PrimitiveComponent Object Reference") (OtherBodyIndex :type Integer) (bFromSweep :type Boolean) (SweepResult :type "HitResult Structure (by ref)"))
  (if (== (`GameplayStatics.GetObjectClass` OtherActor) "/Game/Character/BP_Player_Character.BP_Player_Character_C")
    (`/Engine/EditorBlueprintResources/StandardMacros.DoOnce` false
      (:`Completed`
        (`/Engine/EditorBlueprintResources/StandardMacros.DoOnce` false
          (:`Completed`
            (set `self.PlayerRef` OtherActor)
            (switch `/Game/Hugo/Blueprints/Upgrades/Enum_Upgrades` (`self.ListOfUpgrades`)
              (:`NewEnumerator0`
                (message `/Game/Hugo/Interfaces/BI_Upgrade.BackwardsBullet` (`GameplayStatics.GetGameMode`))
                (message `/Game/Hugo/Interfaces/BI_Upgrade.UpdateUI` (`self.UI_Ref`) "Backwards Bullet!  \nAutomatically shoot A big bullet behind you!  \nYou don't have to think, just destroy!")
                (`Widget.SetVisibility` (`self.UI_Ref`) "Visible")
                (`KismetSystemLibrary.Delay` (`self.TimeForShowingUpgradeInfo`))
                (`Widget.SetVisibility` (`self.UI_Ref`) "Collapsed"))
              (:`NewEnumerator1`
                (message `/Game/Hugo/Interfaces/BI_Upgrade.SpeedBoost` (`GameplayStatics.GetGameMode`) (`self.SpeedBoostProcent`))
                (message `/Game/Hugo/Interfaces/BI_Upgrade.UpdateUI` (`self.UI_Ref`) "Woooo! 30% speed boost")
                (`Widget.SetVisibility` (`self.UI_Ref`) "Visible")
                (`KismetSystemLibrary.Delay` (`self.TimeForShowingUpgradeInfo`))
                (`Widget.SetVisibility` (`self.UI_Ref`) "Collapsed"))
              (:`NewEnumerator3`
                (message `/Game/Hugo/Interfaces/BI_Upgrade.Shield` (`GameplayStatics.GetGameMode`))
                (message `/Game/Hugo/Interfaces/BI_Upgrade.UpdateUI` (`self.UI_Ref`) "Aaawwwhh! A shield! Sweet!  \nIt can break though... but you'll get it back after some time")
                (`Widget.SetVisibility` (`self.UI_Ref`) "Visible")
                (`KismetSystemLibrary.Delay` (`self.TimeForShowingUpgradeInfo`))
                (`Widget.SetVisibility` (`self.UI_Ref`) "Collapsed"))
              (:`NewEnumerator4`
                (message `/Game/Hugo/Interfaces/BI_Upgrade.StrongerBullets` (`GameplayStatics.GetGameMode`) (`self.ProcentForBulletUpgrade`))
                (message `/Game/Hugo/Interfaces/BI_Upgrade.UpdateUI` (`self.UI_Ref`) "Stronger Bullets! \nThe less life you have, \nthe stronger they are.  \nIts amazing!")
                (`Widget.SetVisibility` (`self.UI_Ref`) "Visible")
                (`KismetSystemLibrary.Delay` (`self.TimeForShowingUpgradeInfo`))
                (`Widget.SetVisibility` (`self.UI_Ref`) "Collapsed")))))))))

(fn `SetUpWidgets`
  (bind _returnvalue (`|CreateWidget` "/Game/Hugo/Widgets/BW_Upgrade.BW_Upgrade_C"))
  (bind _output_get (set `self.UI_Ref` _returnvalue))
  (`UserWidget.AddToViewport` _output_get 0)
  (`Widget.SetVisibility` _output_get "Collapsed"))

(fn `UserConstructionScript`)