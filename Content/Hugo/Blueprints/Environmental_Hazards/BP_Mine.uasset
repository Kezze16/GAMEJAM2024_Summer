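; Proximity mine hazard that launches in a random direction on spawn and arms after a short delay by enlarging its trigger sphere.
; An overlap beeps and, if armed, detonates after a delay, while Explosion and DealDamage events detonate it regardless of arming.
; Deploy plays a sound, sphere-traces the blast radius and, inside the hit loop, sends damage messages, deregisters from its parent spawner and destroys itself.
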(event `self.ReceiveBeginPlay`
  (`self.SetCollisionRadiusAndReadyToDeploy`)
  (`self.ShootRandomDirection`))

(event `SetCollisionRadiusAndReadyToDeploy`
  (`KismetSystemLibrary.Delay` 1.0)
  (`SphereComponent.SetSphereRadius` (`self.Collision`) (`self.CollisionRadius`) true)
  (set `self.isReadyToDeploy` true))

(event `self.Collision.OnComponentBeginOverlap`
  (params (OverlappedComponent :type "PrimitiveComponent Object Reference") (OtherActor :type "Actor Object Reference") (OtherComp :type "PrimitiveComponent Object Reference") (OtherBodyIndex :type Integer) (bFromSweep :type Boolean) (SweepResult :type "HitResult Structure (by ref)"))
  (`GameplayStatics.SpawnSoundAtLocation` "/Game/Sound/Hazard/Bip.Bip" (`SceneComponent.K2_GetComponentLocation` (`self.StaticMesh`)) (struct) 1.0 1.0 0.0 null null)
  (`KismetSystemLibrary.Delay` (`self.TimeBeforeDeploy`))
  (if (`self.isReadyToDeploy`)
    (`self.Deploy`)))

(event `/Game/Hugo/Interfaces/BI_MinesAndSpawner.ParentSpawnerRef`
  (params (Spawner :type "Actor Object Reference"))
  (set `self.ParentSpawner` Spawner))

(event `ShootRandomDirection`
  (bind (_returnvalue_x _returnvalue_y) (`KismetMathLibrary.BreakVector` (`SceneComponent.GetForwardVector` (`self.StaticMesh`))))
  (bind _returnvalue (`KismetMathLibrary.RandomFloatInRange` (`self.MinimumSpeed`) (`self.MaximumSpeed`)))
  (`self.K2_SetActorRotation` (`KismetMathLibrary.MakeRotator` 0.0 0.0 (`KismetMathLibrary.RandomFloatInRange` 0.0 360.0)))
  (`ProjectileMovementComponent.SetVelocityInLocalSpace` (`self.ProjectileMovement`) (`KismetMathLibrary.MakeVector` (* _returnvalue_x _returnvalue) (* _returnvalue_y _returnvalue) 650.0)))

(event `/Game/Hugo/Interfaces/BI_Damage.Explosion`
  (params (PotentialDamage :type "Float (double-precision)"))
  (`KismetSystemLibrary.Delay` (`self.TimeBeforeDeploy`))
  (`self.Deploy`))

(event `/Game/Hugo/Interfaces/BI_Damage.DealDamage`
  (params (AmountOfDamage :type "Float (double-precision)"))
  (`KismetSystemLibrary.Delay` (`self.TimeBeforeDeploy`))
  (`self.Deploy`))

(event `/Game/Hugo/Interfaces/BI_MinesAndSpawner.ParentDead`
  (set `self.ParentSpawner` null))

(fn `Deploy`
  (bind _returnvalue (`SceneComponent.K2_GetComponentLocation` (`self.StaticMesh`)))
  (`GameplayStatics.PlaySoundAtLocation` "/Game/Sound/Hazard/Explosion.Explosion" (`SceneComponent.K2_GetComponentLocation` (`self.StaticMesh`)) (struct) 1.0 1.0 0.0 null null null null)
  (bind _outhits (`KismetSystemLibrary.SphereTraceMulti` :`Start` _returnvalue :`End` _returnvalue :`Radius` (`self.Explosion Radius`) :`TraceChannel` "TraceTypeQuery3" :`DrawDebugType` "ForDuration"))
  (for _array_element _outhits
    (message `/Game/Hugo/Interfaces/BI_Damage.Explosion` (`.HitActor` (`GameplayStatics.BreakHitResult` _array_element)) (`self.Damage`))
    (message `/Game/Hugo/Interfaces/BI_MinesAndSpawner.RemoveMineFromArray` (`self.ParentSpawner`) self)
    (`self.K2_DestroyActor`)))

(fn `UserConstructionScript`)