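; BP_ExplosiveSpaceBarrel is an environmental hazard that starts detonating when something overlaps its box trigger.
; A timeline, rescaled to the configured fuse time, swells the mesh toward a multiplied size as a visual countdown.
; When it finishes, a debug-drawn sphere trace at the mesh sends an explosion message with damage for each hit, then the barrel destroys itself.
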(event `self.ReceiveBeginPlay`
  (bind _timebeforedetonate (`self.TimeBeforeDetonate`))
  (`BoxComponent.SetBoxExtent` (`self.Box`) (`self.BoxCollisionExtent`) true)
  (`TimelineComponent.SetPlayRate` _timebeforedetonate (/ (`TimelineComponent.GetTimelineLength` _timebeforedetonate) (`self.TimeBeforeDetonateSeconds`)))
  (bind _output_get (set `self.NormalSize` (`SceneComponent.K2_GetComponentScale` (`self.StaticMesh`))))
  (set `self.MaxMeshSize` (* _output_get (`self.SizeMultiplier`))))

(event `self.Box.OnComponentBeginOverlap`
  (params (OverlappedComponent :type "PrimitiveComponent Object Reference") (OtherActor :type "Actor Object Reference") (OtherComp :type "PrimitiveComponent Object Reference") (OtherBodyIndex :type Integer) (bFromSweep :type Boolean) (SweepResult :type "HitResult Structure (by ref)"))
  (`self.StartDetonating`))

(event `StartDetonating`
  (bind (_direction _alphan) (`Timeline|TimeBeforeDetonate`)
    (:`Update`
      (`SceneComponent.SetWorldScale3D` (`self.StaticMesh`) (`KismetMathLibrary.VLerp` (`self.NormalSize`) (`self.MaxMeshSize`) _alphan)))
    (:`Finished`
      (`self.Detonate`))))

(event `Detonate`
  (`self.Eplosion`)
  (`self.K2_DestroyActor`))

(fn `Eplosion`
  (bind _returnvalue (`SceneComponent.K2_GetComponentLocation` (`self.StaticMesh`)))
  (bind _outhits (`KismetSystemLibrary.SphereTraceMulti` :`Start` _returnvalue :`End` _returnvalue :`Radius` (`self.ExplosionRadius`) :`TraceChannel` "TraceTypeQuery3" :`DrawDebugType` "ForDuration"))
  (for _array_element _outhits
    (message `/Game/Hugo/Interfaces/BI_Damage.Explosion` (`.HitActor` (`GameplayStatics.BreakHitResult` _array_element)) (`self.Damage`))))

(fn `UserConstructionScript`)