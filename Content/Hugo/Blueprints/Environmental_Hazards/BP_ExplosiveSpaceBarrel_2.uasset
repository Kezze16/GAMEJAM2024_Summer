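; Explosive space barrel hazard that starts a timed detonation when its box is overlapped or its DealDamage or Explosion events fire.
; A timeline, rescaled to the configured fuse time, swells the mesh and drives a dynamic-material progress indicator on a plane sized to the blast radius.
; When it finishes, a multi-sphere trace sends ExplosionMessage with the damage value to hit actors, then the barrel destroys itself.
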(event `Update Plane Scale`
  (`SceneComponent.SetRelativeScale3D` (`self.Plane`) (`KismetMathLibrary.Conv_DoubleToVector` (* (* (`self.ExplosionRadius`) 0.01) 2.0))))

(event `self.ReceiveBeginPlay`
  (bind _timebeforedetonate (`self.TimeBeforeDetonate`))
  (`self.Update Plane Scale`)
  (`BoxComponent.SetBoxExtent` (`self.Box`) (`self.BoxCollisionExtent`) true)
  (`TimelineComponent.SetPlayRate` _timebeforedetonate (/ (`TimelineComponent.GetTimelineLength` _timebeforedetonate) (`self.TimeBeforeDetonateSeconds`)))
  (bind _output_get (set `self.NormalSize` (`SceneComponent.K2_GetComponentScale` (`self.StaticMesh`))))
  (set `self.MaxMeshSize` (* _output_get (`self.SizeMultiplier`))))

(event `self.Box.OnComponentBeginOverlap`
  (params (OverlappedComponent :type "PrimitiveComponent Object Reference") (OtherActor :type "Actor Object Reference") (OtherComp :type "PrimitiveComponent Object Reference") (OtherBodyIndex :type Integer) (bFromSweep :type Boolean) (SweepResult :type "HitResult Structure (by ref)"))
  (`self.StartDetonating` :!label _label))

(event `/Game/Hugo/Interfaces/BI_Damage.DealDamage`
  (params (AmountOfDamage :type "Float (double-precision)"))
  (goto _label))

(event `/Game/Hugo/Interfaces/BI_Damage.Explosion`
  (params (PotentialDamage :type "Float (double-precision)"))
  (goto _label))

(event `StartDetonating`
  (`MaterialInstanceDynamic.SetScalarParameterValue` (`self.ExplosionBar`) "Percent" 0.5)
  (bind (_direction _alphan _time) (`Timeline|TimeBeforeDetonate`)
    (:`Update`
      (`SceneComponent.SetWorldScale3D` (`self.StaticMesh`) (`KismetMathLibrary.VLerp` (`self.NormalSize`) (`self.MaxMeshSize`) _alphan))
      (`MaterialInstanceDynamic.SetScalarParameterValue` (`self.ExplosionBar`) "Radius" (`KismetMathLibrary.Lerp` 0.0 0.5 _time)))
    (:`Finished`
      (`self.Detonate`))))

(event `Detonate`
  (`self.Eplosion`)
  (`self.K2_DestroyActor`))

(fn `CreateProgressionBar`
  (bind _returnvalue (`KismetMaterialLibrary.CreateDynamicMaterialInstance` "/Game/Hugo/Blueprints/Environmental_Hazards/M_Explosion_Bar2.M_Explosion_Bar2"))
  (bind _output_get (set `self.ExplosionBar` _returnvalue))
  (`PrimitiveComponent.SetMaterial` (`self.Plane`) 0 _output_get)
  (`MaterialInstanceDynamic.SetScalarParameterValue` (`self.ExplosionBar`) "Radius" 0.0))

(fn `Eplosion`
  (bind _returnvalue (`SceneComponent.K2_GetComponentLocation` (`self.StaticMesh`)))
  (bind _outhits (`KismetSystemLibrary.SphereTraceMulti` :`Start` _returnvalue :`End` _returnvalue :`Radius` (`self.ExplosionRadius`) :`TraceChannel` "TraceTypeQuery3" :`DrawTime` 1.0))
  (for _array_element _outhits
    (message `/Game/Hugo/Interfaces/BI_Damage.Explosion` (`.HitActor` (`GameplayStatics.BreakHitResult` _array_element)) (`self.Damage`))))

(fn `UserConstructionScript`
  (`self.CreateProgressionBar`))