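; Rotating laser cannon hazard that turns its mesh by a set yaw step, pauses, and repeats from BeginPlay.
; Timelines, with play rates scaled from duration variables, drive the pause, rotation lerp and beam.
; While stationary, the beam repeatedly sphere-traces forward from SpawningPoint with debug drawing, sending damage messages and tracking hit actors to limit repeat hits.
; ShootLazer and FirstTimeTuchingLazerCheck are trace helpers the event graph never calls.
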(event `self.ReceiveBeginPlay`
  (bind _rotatingmesh (`self.RotatingMesh`))
  (bind _lazeractivetime (`self.LazerActiveTime`))
  (bind _intervalwhenrotating (`self.IntervalWhenRotating`))
  (`TimelineComponent.SetPlayRate` _intervalwhenrotating (/ (`TimelineComponent.GetTimelineLength` _intervalwhenrotating) (`self.SecondsForIntervalTimeLine`)))
  (`TimelineComponent.SetPlayRate` _rotatingmesh (/ (`TimelineComponent.GetTimelineLength` _rotatingmesh) (`self.RotatingSpeed`)))
  (`TimelineComponent.SetPlayRate` _lazeractivetime (/ (`TimelineComponent.GetTimelineLength` _lazeractivetime) (`self.LazerActiveSeconds`)))
  (`self.Rotating`))

(event `Rotating`
  (bind _returnvalue (`SceneComponent.K2_GetComponentRotation` (`self.StaticMesh1`)))
  (`Timeline|IntervalWhenRotating` :!via `PlayFromStart`
    (:`Finished`
      (set `self.CurrentRotation` _returnvalue)
      (set `self.RotationGoal` (`KismetMathLibrary.MakeRotator` (.roll _returnvalue) (.pitch _returnvalue) (+ (.yaw _returnvalue) (`self.RotateAngle`))))
      (set `self.isRotating` true)
      (`KismetArrayLibrary.Array_Clear` (`self.ArrayOfAlreadyHitTargets`))
      (bind (_direction _alpha) (`Timeline|RotatingMesh` :!via `PlayFromStart`)
        (:`Update`
          (`SceneComponent.K2_SetWorldRotation` (`self.StaticMesh1`) (`KismetMathLibrary.RLerp` (`self.CurrentRotation`) (`self.RotationGoal`) _alpha) false false))
        (:`Finished`
          (set `self.isRotating` false)
          (`self.Shoot`)
          (`self.Rotating`))))))

(event `Shoot`
  (bind _spawningpoint (`self.SpawningPoint`))
  (bind _arrayofalreadyhittargets (`self.ArrayOfAlreadyHitTargets`))
  (bind _returnvalue (`SceneComponent.K2_GetComponentLocation` _spawningpoint))
  (if (not (`self.isRotating`))
    (`Timeline|LazerActiveTime` :!via `PlayFromStart`
      (:`Update`
        (if (not (`self.isRotating`))
          (bind _outhits (`KismetSystemLibrary.SphereTraceMulti` :`Start` _returnvalue :`End` (+ _returnvalue (* (`KismetMathLibrary.GetForwardVector` (`SceneComponent.K2_GetComponentRotation` _spawningpoint)) (`self.LazerDistance`))) :`Radius` (`self.LazerRadius`) :`TraceChannel` "TraceTypeQuery3" :`DrawDebugType` "ForOneFrame"))
          (if (`KismetArrayLibrary.Array_IsEmpty` _outhits)
            (`KismetArrayLibrary.Array_Clear` (`self.ArrayOfAlreadyHitTargets`))
            (else
              (for _array_element _outhits
                (bind (_bblockinghit _binitialoverlap _time _distance _location _impactpoint _normal _impactnormal _physmat _hitactor) (`GameplayStatics.BreakHitResult` _array_element))
                (if (not (`KismetArrayLibrary.Array_IsValidIndex` _arrayofalreadyhittargets (`KismetArrayLibrary.Array_Find` _arrayofalreadyhittargets _hitactor)))
                  (`KismetArrayLibrary.Array_AddUnique` (`self.ArrayOfAlreadyHitTargets`) _hitactor)
                  (message `/Game/Hugo/Interfaces/BI_Damage.DealDamage` _hitactor (`self.Damage`))
                  (`KismetSystemLibrary.Delay` (`self.LazerActiveSeconds`))
                  (`KismetArrayLibrary.Array_RemoveItem` (`self.ArrayOfAlreadyHitTargets`) _hitactor)))))))
      (:`Finished`
        (`self.Shoot`)))))

(fn `FirstTimeTuchingLazerCheck`
  (bind _spawningpoint (`self.SpawningPoint`))
  (bind _arrayofalreadyhittargets (`self.ArrayOfAlreadyHitTargets`))
  (bind _returnvalue (`SceneComponent.K2_GetComponentLocation` _spawningpoint))
  (bind _outhits (`KismetSystemLibrary.SphereTraceMulti` :`Start` _returnvalue :`End` (+ _returnvalue (* (`KismetMathLibrary.GetForwardVector` (`SceneComponent.K2_GetComponentRotation` _spawningpoint)) (`self.LazerDistance`))) :`Radius` (`self.LazerRadius`) :`TraceChannel` "TraceTypeQuery3" :`DrawDebugType` "ForDuration"))
  (for _array_element _outhits
    (bind (_bblockinghit _binitialoverlap _time _distance _location _impactpoint _normal _impactnormal _physmat _hitactor) (`GameplayStatics.BreakHitResult` _array_element))
    (if (not (`KismetArrayLibrary.Array_IsValidIndex` _arrayofalreadyhittargets (`KismetArrayLibrary.Array_Find` _arrayofalreadyhittargets _hitactor)))
      (`KismetArrayLibrary.Array_AddUnique` (`self.ArrayOfAlreadyHitTargets`) _hitactor)
      (message `/Game/Hugo/Interfaces/BI_Damage.DealDamage` _hitactor (`self.Damage`)))))

(fn `ShootLazer`
  (bind _spawningpoint (`self.SpawningPoint`))
  (bind _returnvalue (`SceneComponent.K2_GetComponentLocation` _spawningpoint))
  (bind _outhits (`KismetSystemLibrary.SphereTraceMulti` :`Start` _returnvalue :`End` (+ _returnvalue (* (`KismetMathLibrary.GetForwardVector` (`SceneComponent.K2_GetComponentRotation` _spawningpoint)) (`self.LazerDistance`))) :`Radius` (`self.LazerRadius`) :`TraceChannel` "TraceTypeQuery3" :`DrawDebugType` "ForDuration"))
  (for _array_element _outhits
    (message `/Game/Hugo/Interfaces/BI_Damage.DealDamage` (`.HitActor` (`GameplayStatics.BreakHitResult` _array_element)) 0.0)))

(fn `UserConstructionScript`)