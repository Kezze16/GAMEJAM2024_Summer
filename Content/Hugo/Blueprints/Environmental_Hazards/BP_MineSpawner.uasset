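; BP_MineSpawner is a destructible environmental hazard that spawns BP_Mine actors at its spawn point on a timed interval.
; A timeline scaled to the interval drives spawning until the mine cap is reached, and removing a mine from the tracked array restarts it.
; Each mine receives a reference to its spawner.
; Damage briefly shrinks the body and accumulates until maximum durability, when the spawner notifies its mines and destroys itself.
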(event `self.ReceiveBeginPlay`
  (bind _intervaltimeline (`self.IntervalTimeline`))
  (`TimelineComponent.SetPlayRate` _intervaltimeline (/ (`TimelineComponent.GetTimelineLength` _intervaltimeline) (`self.IntervalSecond`)))
  (`self.TimeIntervallForSpawning`))

(event `TimeIntervallForSpawning`
  (`Timeline|IntervalTimeline` :!via `PlayFromStart`
    (:`Finished`
      (`self.SpawnMine`)
      (if (< (`KismetArrayLibrary.Array_Length` (`self.ArrayOfMines`)) (`self.AmountOfMinesAbleToExist`))
        (`self.TimeIntervallForSpawning`)
        (`GameplayStatics.PlaySound2D` "/Game/Sound/Hazard/MineDepoly.MineDepoly" 1.0 1.0 0.0 null null)))))

(event `/Game/Hugo/Interfaces/BI_MinesAndSpawner.RemoveMineFromArray`
  (params (MineRef :type "Actor Object Reference"))
  (`KismetArrayLibrary.Array_RemoveItem` (`self.ArrayOfMines`) MineRef)
  (`self.TimeIntervallForSpawning`))

(event `/Game/Hugo/Interfaces/BI_Damage.DealDamage`
  (params (AmountOfDamage :type "Float (double-precision)"))
  (`self.Hit`)
  (bind _output_get (set `self.BeenHit` (+ (`self.BeenHit`) AmountOfDamage)))
  (if (>= _output_get (`self.MaxDurability`))
    (for _array_element (`self.ArrayOfMines`)
      (message `/Game/Hugo/Interfaces/BI_MinesAndSpawner.ParentDead` _array_element)
      (`self.K2_DestroyActor`))))

(event `Hit`
  (bind _body (`self.Body`))
  (bind _body_2 (`self.Body`))
  (`KismetSystemLibrary.Delay` 0.1)
  (`SceneComponent.SetWorldScale3D` _body (- (`SceneComponent.RelativeScale3D` _body) (0.2 0.2 0.2)))
  (`KismetSystemLibrary.Delay` 0.1)
  (`SceneComponent.SetWorldScale3D` _body_2 (+ (`SceneComponent.RelativeScale3D` _body_2) (0.2 0.2 0.2))))

(fn `SpawnMine`
  (bind _spawnpoint (`self.SpawnPoint`))
  (bind _returnvalue (`|SpawnActorFromClass` "/Game/Hugo/Blueprints/Environmental_Hazards/BP_Mine.BP_Mine_C" (`KismetMathLibrary.MakeTransform` (`SceneComponent.K2_GetComponentLocation` _spawnpoint) (`SceneComponent.K2_GetComponentRotation` _spawnpoint)) "Undefined" "MultiplyWithRoot" null null))
  (`KismetArrayLibrary.Array_AddUnique` (`self.ArrayOfMines`) _returnvalue)
  (message `/Game/Hugo/Interfaces/BI_MinesAndSpawner.ParentSpawnerRef` _returnvalue self))

(fn `UserConstructionScript`)