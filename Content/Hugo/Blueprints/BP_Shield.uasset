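; BP_Shield is a destructible shield actor that absorbs damage for an owner set through ShieldOwner.
; DealDamage, also fed by Explosion, lowers clamped durability, notifies the owner of each hit and starts DestroyShield at zero.
; DestroyShield re-calls itself through delays as a counted flicker, then reports the break to the owner and destroys the actor.
; Both flicker visibility calls set the mesh visible, so it never actually hides.
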(event `self.ReceiveBeginPlay`
  (set `self.CurrentDurability` (`self.MaxDurability`)))

(event `/Game/Hugo/Interfaces/BI_Damage.DealDamage`
  (params (AmountOfDamage :type "Float (double-precision)"))
  (set `self.CurrentDurability` (`KismetMathLibrary.FClamp` (- (`self.CurrentDurability`) AmountOfDamage) 0.0 (`self.MaxDurability`)))
  (message `/Game/Hugo/Interfaces/BI_Shield.ShieldGotHit` (`self.OwnerRef`))
  (if (<= (`self.CurrentDurability`) 0.0)
    (`self.DestroyShield`)))

(event `/Game/Hugo/Interfaces/BI_Damage.Explosion`
  (params (PotentialDamage :type "Float (double-precision)"))
  (`/Game/Hugo/Interfaces/BI_Damage.DealDamage` PotentialDamage))

(event `DestroyShield`
  (bind _mesh (`self.Mesh`))
  (`SceneComponent.SetVisibility` _mesh true false)
  (`KismetSystemLibrary.Delay` 0.2)
  (`SceneComponent.SetVisibility` _mesh true false)
  (`KismetSystemLibrary.Delay` 0.2)
  (`self.DestroyShield`)
  (bind _result (`/Engine/EditorBlueprintResources/StandardMacros.IncrementInt` (`self.FlickerCounter`))
    (:`  `
      (if (== _result (`self.FlickerAamountWhenBeingDestroyed`))
        (message `/Game/Hugo/Interfaces/BI_Shield.ShieldBroke` (`self.OwnerRef`))
        (`self.K2_DestroyActor`)))))

(event `/Game/Hugo/Interfaces/BI_Shield.ShieldOwner`
  (params (Owner :type "Actor Object Reference"))
  (set `self.OwnerRef` Owner))

(fn `UserConstructionScript`)